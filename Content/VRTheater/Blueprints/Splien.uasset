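; Spline path Blueprint that moves a referenced actor along its spline in an endless loop.
; BeginPlay divides the spline length into AnimationSteps, then a self-calling event eases the actor's root to each successive point with latent MoveComponentTo, wrapping at the end.
; Rotation follows the spline with pitch and yaw offsets, while roll adds a clock-seconds-based spin and RotateX is unused.
; The construction script toggles spline debug drawing.
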(event Custom|MoveActorToNextPoint
  (bind _spline (Variables|Default|GetSpline))
  (bind _result (Math|Float|IncrementFloat (Variables|Default|GetAnimationIndex))
    (:%20%20
      (if (< _result (Variables|Default|GetAnimationSteps))
        (Variables|Default|SetAnimationIndex _result)
        (else
          (Variables|Default|SetAnimationIndex 0.0)))
      (Components|MoveComponentTo (Variables|/Script/Engine.Actor|GetRootComponent (Variables|Default|GetActor)) (Spline|GetLocationatDistanceAlongSpline _spline (* (Variables|Default|GetStepDistance) (Variables|Default|GetAnimationIndex)) "World") (Math|Rotator|MakeRotator (+ (.roll (Spline|GetRotationatDistanceAlongSpline _spline (* (Variables|Default|GetStepDistance) (Variables|Default|GetAnimationIndex)) "World")) (* (Class|KismetMathLibrary|GetSecond) 10)) (+ (.pitch (Spline|GetRotationatDistanceAlongSpline _spline (* (Variables|Default|GetStepDistance) (Variables|Default|GetAnimationIndex)) "World")) (Variables|Default|GetRotateY)) (+ (.yaw (Spline|GetRotationatDistanceAlongSpline _spline (* (Variables|Default|GetStepDistance) (Variables|Default|GetAnimationIndex)) "World")) (Variables|Default|GetRotateZ))) false false (Variables|Default|GetOver%20Time) false)
      (CallFunction|MoveActortoNextPoint))))

(event EventBeginPlay
  (Variables|Default|SetStepDistance (/ (Spline|GetSplineLength (Variables|Default|GetSpline)) (Variables|Default|GetAnimationSteps)))
  (CallFunction|MoveActortoNextPoint))

(fn ConstructionScript
  (Class|SplineComponent|SetDrawDebug (Variables|Default|GetSpline) (Variables|Default|GetShow%20in%20Game)))