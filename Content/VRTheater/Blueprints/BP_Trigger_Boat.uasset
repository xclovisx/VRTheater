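; Trigger Blueprint for the VR theater that slides a ship mesh along its relative X axis.
; The StartBoat event plays a Timeline whose float track lerps the ship's X offset, rewriting its relative transform at a fixed enlarged scale each update.
; The StartTrigger override only calls the parent with a constant zero count; nothing in this Blueprint calls StartBoat.
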(event Custom|StartBoat
  (bind _boatfloat (Timeline|Timeline Play)
    (:Update
      (Transformation|SetRelativeTransform (Variables|Default|Getmodern_ship_combined_with_pea_pod_0410115947_refine) (Math|Transform|MakeTransform (Math|Vector|MakeVector (Math|Float|Lerp 0.0 -7.6e+03 _boatfloat) 0.0 0.0) "0, 0, 0" "5.000000,5.000000,5.000000") false false))))

(event EventBeginPlay
  (|CallParentFunction) ; This node is disabled and will not be called.\nDrag off pins to build functionality.
)

(fn ConstructionScript
  (|CallParentFunction))

(fn StartTrigger
  (params (TimesTriggerd :type Integer))
  (|CallParentFunction 0))