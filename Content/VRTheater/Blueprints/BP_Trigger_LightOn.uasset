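; BP_Trigger_LightOn is a VR theater trigger that switches on a point light and starts a timer for a set duration.
; StartTrigger overrides the parent without calling it, makes the PointLight visible and starts a one-shot timer of length Duration.
; EndTrigger turns the light's visibility off again, though the timer's bound event is not shown.
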(event EventBeginPlay
  (|CallParentFunction))

(fn ConstructionScript
  (|CallParentFunction))

(fn StartTrigger
  (bind _pointlight (Variables|Default|GetPointLight))
  (Rendering|SetVisibility _pointlight true false)
  (Development|SetHiddeninGame _pointlight false false)
  (Utilities|Time|SetTimerbyEvent (EventDispatchers|CreateEvent :!event EndTrigger) (Variables|Default|GetDuration)))

(fn EndTrigger
  (bind _pointlight (Variables|Default|GetPointLight))
  (Rendering|SetVisibility _pointlight false false)
  (Development|SetHiddeninGame _pointlight false false))